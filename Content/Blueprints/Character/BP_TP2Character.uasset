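; BP_TP2Character is a character Blueprint with a debug-style auto-move toggle and unfinished back-and-forth movement logic.
; Pressing P sets AutoMove to true, while Tick is empty.
; A disconnected authority switch would move the character along its forward vector, flipping MoveForward after two-second delays, with remote instances gated by AutoMove.
; Nothing triggers that branch, so the movement never runs.
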(event `self.ReceiveTick`
  (params (DeltaSeconds :type "Float (single-precision)")))

(event `Key|P`
  (params (Key :type "Key Structure"))
  (:`Pressed`
    (set `self.AutoMove` true)))

(fn `UserConstructionScript`)